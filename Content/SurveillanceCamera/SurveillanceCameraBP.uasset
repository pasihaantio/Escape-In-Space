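; Surveillance camera Blueprint that detects actors tagged Player with a cone and shows its state through a colored decal.
; Cone overlaps set or clear DetectedPlayer, but both begin and end set Status to 1, so nothing here resets it.
; Tick creates a new dynamic decal material each frame, tinted red at Status 1 and green otherwise.
; A separate OnRaiseAlarm event prints a message and calls the alarm dispatcher.
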(event `self.ReceiveBeginPlay`)

(event `self.ReceiveTick`
  (params (DeltaSeconds :type "Float (single-precision)"))
  (bind _returnvalue (`KismetMaterialLibrary.CreateDynamicMaterialInstance` "/Game/SurveillanceCamera/TestDecal.TestDecal"))
  (`DecalComponent.SetDecalMaterial` (`self.Decal`) _returnvalue)
  (if (== (`self.Status`) 1)
    (`MaterialInstanceDynamic.SetVectorParameterValue` _returnvalue "TestDecalC" (make `LinearColor` 1.0))
    (else
      (`MaterialInstanceDynamic.SetVectorParameterValue` _returnvalue "TestDecalC" (make `LinearColor` 0.0 1.0)))))

(event `self.SurveillanceCone.OnComponentBeginOverlap`
  (params (OverlappedComponent :type "PrimitiveComponent Object Reference") (OtherActor :type "Actor Object Reference") (OtherComp :type "PrimitiveComponent Object Reference") (OtherBodyIndex :type Integer) (bFromSweep :type Boolean) (SweepResult :type "HitResult Structure (by ref)"))
  (if (`self.ActorHasTag` OtherActor "Player")
    (set `self.Status` 1)
    (set `self.detectedPlayer` OtherActor)))

(event `self.SurveillanceCone.OnComponentEndOverlap`
  (params (OverlappedComponent :type "PrimitiveComponent Object Reference") (OtherActor :type "Actor Object Reference") (OtherComp :type "PrimitiveComponent Object Reference") (OtherBodyIndex :type Integer))
  (if (`self.ActorHasTag` OtherActor "Player")
    (set `self.Status` 1)
    (set `self.detectedPlayer` null)))

(event `self.OnRaiseAlarm`
  (`KismetSystemLibrary.PrintString` "Alarm")
  (`self.AlarmDispatch`))

(fn `UserConstructionScript`)